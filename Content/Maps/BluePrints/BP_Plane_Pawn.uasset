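; BP_Plane_Pawn is a player-controlled plane that constantly flies forward along its local axis.
; Tick applies frame-rate-scaled movement and calls RotatePropeller to spin both propellers, reaching the right one twice per frame.
; Pitch input rotates the actor by the clamped axis value, while Roll clamps a constant zero, so it currently has no effect.
; An unconnected world-offset movement alternative remains unused.
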(event `self.ReceiveTick`
  (params (DeltaSeconds :type "Float (single-precision)"))
  (`|ExecutionSequence`
    (:`then_0`
      ;[1 1 1] 앞으로 이동
      (`self.K2_AddActorLocalOffset` (`KismetMathLibrary.MakeVector` (* (`self.MoveSpeed`) (`GameplayStatics.GetWorldDeltaSeconds`))))
      (`KismetSystemLibrary.Delay` 3.0))
    (:`then_1`
      ;[1 1 1] 왼쪽 프로펠러 회전
      (`self.Rotate Propeller` (`self.Left`))
      ;[1 1 1] 오른쪽 프로펠러 회전
      (`self.Rotate Propeller` (`self.Right`) :!label _label))
    (:`then_2`
      (goto _label))))

(event `InputAxis|Pitch`
  (params (AxisValue :type "Float (single-precision)"))
  ;[1 1 1] 피치 회전
  (`self.K2_AddActorLocalRotation` (`KismetMathLibrary.MakeRotator` 0.0 (* (`KismetMathLibrary.FClamp` AxisValue -1.0) (`GameplayStatics.GetWorldDeltaSeconds`) (`self.PlayerRotateSpeed`)))))

(event `InputAxis|Roll`
  (params (AxisValue :type "Float (single-precision)"))
  ;[1 1 1] 롤 회전
  (`self.K2_AddActorLocalRotation` (`KismetMathLibrary.MakeRotator` (* (`KismetMathLibrary.FClamp` 0.0 -1.0) (`GameplayStatics.GetWorldDeltaSeconds`) (`self.PlayerRotateSpeed`)))))

(fn `Rotate Propeller`
  (params (self2 :type "StaticMeshComponent Object Reference"))
  (locals (NewLocalVar :type "Float (double-precision)"))
  (`SceneComponent.K2_AddRelativeRotation` self2 (`KismetMathLibrary.MakeRotator` (* (`GameplayStatics.GetWorldDeltaSeconds`) (`self.RollPropeller`))) false false))

(fn `UserConstructionScript`)